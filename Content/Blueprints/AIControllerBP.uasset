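; AI controller Blueprint that sets up patrol behavior for a ThirdPersonCharacter pawn.
; On BeginPlay it initializes the PatrolData blackboard, seeds it through UpdatePatrol, then runs the Patrol behavior tree.
; UpdatePatrol writes the pawn's first patrol point as the Waypoint key and a fixed WaitTime, doing nothing if the pawn cast fails.
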(event EventBeginPlay
  (Development|PrintString "AIController up and running")
  ;[1 1 1] Setup Blackboard
  (bind _blackboardcomponent (Class|AIController|UseBlackboard "/Game/Behaviors/PatrolData.PatrolData"))
  (CallFunction|UpdatePatrol _blackboardcomponent)
  (AI|RunBehaviorTree "/Game/Behaviors/Patrol.Patrol"))

(event EventTick
  (params (DeltaSeconds :type Float%20%28single-precision%29)))

(fn ConstructionScript)

(fn UpdatePatrol
  (params (blackboard :type Blackboard%20Component%20Object%20Reference))
  (bind _asthird_person_character (Utilities|Casting|CastToThirdPersonCharacter (Pawn|GetControlledPawn)))
  (AI|Components|Blackboard|SetValueasObject blackboard (Utilities|Name|MakeLiteralName "Waypoint") (Utilities|Array|Get(acopy) (Variables|/Game/ThirdPersonCPP/Blueprints/ThirdPersonCharacter.ThirdPersonCharacter_C|GetPatrolPoints _asthird_person_character)))
  (AI|Components|Blackboard|SetValueasFloat blackboard (Utilities|Name|MakeLiteralName "WaitTime") 1.2))